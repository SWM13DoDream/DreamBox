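; BP_TransitionLogo is a transition actor that animates a logo shown through its LogoWidgetComponent.
; On BeginPlay it casts the component's widget to W_TransitionLogo and caches the reference.
; PlayLogoAnimation forwards its begin flag to the widget's PlayAppearAnim when GetLogoAnimationIsSet passes for that flag.
; PlayLogoDisappearAnim reuses the same event with the flag set to false.
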(event EventBeginPlay
  (bind _asw_transition_logo (Utilities|Casting|CastToW_TransitionLogo (UserInterface|GetWidget (Variables|Default|GetLogoWidgetComponent))))
  (Variables|Default|SetTransitionLogoRef _asw_transition_logo))

(event EventPlayLogoAnimation
  (params (bIsBeginAnim :type Boolean))
  (if (Class|TransitionLogo|GetLogoAnimationIsSet bIsBeginAnim)
    (Default|PlayAppearAnim (Variables|Default|GetTransitionLogoRef) bIsBeginAnim)))

(event EventPlayLogoDisappearAnim
  (Class|TransitionLogo|PlayLogoAnimation false))

(fn ConstructionScript)