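; Actor that hosts the Astronaut game's mission selection panel and waiting-for-player screen as widget components with background music.
; On BeginPlay it caches both widgets and hands each a reference to itself.
; External events animate the screens in and out with delayed hiding, fade music, and lock the LEM or CSM choice.
; Ending the wait flags the GameMode as InMission, then reveals mission selection.
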(event Custom|PlayBGM
  (Audio|Components|Audio|FadeIn (Variables|Default|GetBackgroundMusic) 1.5 1.0 0.0 "Linear" :!class /Script/Engine.AudioComponent))

(event Custom|StopBGM
  (Audio|Components|Audio|FadeOut (Variables|Default|GetBackgroundMusic) 3.0 0.0 "Linear" :!class /Script/Engine.AudioComponent))

(event EventDeactivate
  (Default|Deanimate (Variables|Default|GetCastedWidget))
  (CallFunction|StopBGM)
  (Utilities|FlowControl|Delay 1.5)
  (Development|SetHiddeninGame (Variables|Default|GetMainWidget) true false))

(event EventLockMission
  (params (Mission :type Integer))
  (bind _castedwidget (Variables|Default|GetCastedWidget))
  (if (== Mission (Math|Conversions|ToInteger(Byte) (Utilities|Enum|LiteralenumEAstronautMissionType "NONE")))
    (Default|Unlock _castedwidget)
    (elif (== Mission (Math|Conversions|ToInteger(Byte) (Utilities|Enum|LiteralenumEAstronautMissionType "LEM")))
      (Default|LockLEM _castedwidget)
      (else
        (Default|LockCSM _castedwidget)))))

(event EventWaitingforPlayer
  (params (Address :type String))
  (bind _waitingwidget (Variables|Default|GetWaitingWidget))
  (CallFunction|PlayBGM)
  (Development|SetHiddeninGame _waitingwidget false false)
  (Collision|SetCollisionEnabled _waitingwidget "QueryAndPhysics")
  (Default|Animate (Variables|Default|GetCastedSubwidget) Address))

(event EventBeginPlay
  (bind _backgroundmusic (Variables|Default|GetBackgroundMusic))
  (Components|Activation|Activate _backgroundmusic false)
  (Audio|Components|Audio|Stop _backgroundmusic)
  (bind _asw_mission_selection (Utilities|Casting|CastToW_MissionSelection (UserInterface|GetWidget (Variables|Default|GetMainWidget))))
  (bind _output_get (Variables|Default|SetCastedWidget _asw_mission_selection))
  (Variables|/Game/Astronaut/UI/W_MissionSelection.W_MissionSelection_C|SetControlPanel _output_get self)
  (bind _asw_waiting_player (Utilities|Casting|CastToW_WaitingPlayer (UserInterface|GetWidget (Variables|Default|GetWaitingWidget))))
  (bind _output_get_2 (Variables|Default|SetCastedSubwidget _asw_waiting_player))
  (Variables|/Game/Astronaut/UI/W_WaitingPlayer.W_WaitingPlayer_C|SetControlPanel _output_get_2 self))

(event EventActivate
  (CallFunction|PlayBGM)
  (Development|SetHiddeninGame (Variables|Default|GetMainWidget) false false)
  (Default|Animate (Variables|Default|GetCastedWidget)))

(event EventStopWaitingPlayer
  (bind _waitingwidget (Variables|Default|GetWaitingWidget))
  (Default|Deanimate (Variables|Default|GetCastedSubwidget))
  (Collision|SetCollisionEnabled _waitingwidget "NoCollision")
  (bind _asastronaut_gamemode (Utilities|Casting|CastToAstronautGamemode (Game|GetGameMode)))
  (Variables|/Script/DreamBox.AstronautGamemode|SetbInMission _asastronaut_gamemode true)
  (Utilities|FlowControl|Delay 1.0)
  (Development|SetHiddeninGame _waitingwidget true false)
  (Development|SetHiddeninGame (Variables|Default|GetMainWidget) false false)
  (Default|Animate (Variables|Default|GetCastedWidget)))

(fn ConstructionScript)