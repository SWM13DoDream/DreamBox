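; BP_DialogController is an actor that plays timed voice and text dialog for the LEM in the astronaut game.
; Three custom events (intro, mid, approx) each play a 2D sound, then step through sequential D_Dialog data table rows.
; Each row's content goes to SetDialogContent and is held by a Delay for that row's duration, then the text is cleared after the last line.
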(event EventLEMDialogIntro
  (Audio|PlaySound2D "/Game/Astronaut/Sound/SE_LEM_Intro.SE_LEM_Intro" 1.0 1.0 0.0 0 0)
  (bind _returnvalue (Utilities|GetDataTableRow "/Game/Astronaut/Data/D_Dialog.D_Dialog" "LEM_Intro_1")
    (:then
      (Class|DialogController|SetDialogContent (.content _returnvalue))
      (Utilities|FlowControl|Delay (.duration _returnvalue))
      (bind _returnvalue_2 (Utilities|GetDataTableRow "/Game/Astronaut/Data/D_Dialog.D_Dialog" "LEM_Intro_2")
        (:then
          (Class|DialogController|SetDialogContent (.content _returnvalue_2))
          (Utilities|FlowControl|Delay (.duration _returnvalue_2))
          (bind _returnvalue_3 (Utilities|GetDataTableRow "/Game/Astronaut/Data/D_Dialog.D_Dialog" "LEM_Intro_3")
            (:then
              (Class|DialogController|SetDialogContent (.content _returnvalue_3))
              (Utilities|FlowControl|Delay (.duration _returnvalue_3))
              (bind _returnvalue_4 (Utilities|GetDataTableRow "/Game/Astronaut/Data/D_Dialog.D_Dialog" "LEM_Intro_4")
                (:then
                  (Class|DialogController|SetDialogContent (.content _returnvalue_4))
                  (Utilities|FlowControl|Delay (.duration _returnvalue_4))
                  (Class|DialogController|SetDialogContent))))))))))

(event EventLEMDialogMid
  (Audio|PlaySound2D "/Game/Astronaut/Sound/SE_LEM_TimeMiddle.SE_LEM_TimeMiddle" 1.0 1.0 0.0 0 0)
  (bind _returnvalue (Utilities|GetDataTableRow "/Game/Astronaut/Data/D_Dialog.D_Dialog" "LEM_Mid_1")
    (:then
      (Class|DialogController|SetDialogContent (.content _returnvalue))
      (Utilities|FlowControl|Delay (.duration _returnvalue))
      (bind _returnvalue_2 (Utilities|GetDataTableRow "/Game/Astronaut/Data/D_Dialog.D_Dialog" "LEM_Mid_2")
        (:then
          (Class|DialogController|SetDialogContent (.content _returnvalue_2))
          (Utilities|FlowControl|Delay (.duration _returnvalue_2))
          (Class|DialogController|SetDialogContent))))))

(event EventLEMDialogApprox
  (Audio|PlaySound2D "/Game/Astronaut/Sound/SE_LEM_TimeApprox.SE_LEM_TimeApprox" 1.0 1.0 0.0 0 0)
  (bind _returnvalue (Utilities|GetDataTableRow "/Game/Astronaut/Data/D_Dialog.D_Dialog" "LEM_Approx_1")
    (:then
      (Class|DialogController|SetDialogContent (.content _returnvalue))
      (Utilities|FlowControl|Delay (.duration _returnvalue))
      (bind _returnvalue_2 (Utilities|GetDataTableRow "/Game/Astronaut/Data/D_Dialog.D_Dialog" "LEM_Approx_2")
        (:then
          (Class|DialogController|SetDialogContent (.content _returnvalue_2))
          (Utilities|FlowControl|Delay (.duration _returnvalue_2))
          (Class|DialogController|SetDialogContent))))))

(fn ConstructionScript)