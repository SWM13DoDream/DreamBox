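; Astronaut character Blueprint that runs the intro cinematics and chains the tutorial info panels leading into mission selection and movement.
; The initial level sequence plays, pauses for the Trigger panel, then resumes before mission initialization, with a separate cross-fade sequence available.
; A key-to-class map fills one widget component, and each close key opens the next panel, mission selection, or enables movement.
; Test inputs trigger panel closing and CSM or LEM selection.
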(event Custom|Hide%20Info%20Widget
  (bind _infowidget (Variables|Default|GetInfoWidget))
  (Utilities|FlowControl|Delay 0.5)
  (Development|SetHiddeninGame _infowidget true false)
  (Collision|SetCollisionEnabled _infowidget "NoCollision"))

(event EventPlayInitialSequence
  (bind _outactor (Sequencer|Player|CreateLevelSequencePlayer "/Game/Astronaut/Sequencer/SQ_InitialAnim.SQ_InitialAnim"))
  (bind _output_get (Variables|Default|SetInitialSequenceRef (Variables|/Script/LevelSequence.LevelSequenceActor|GetSequencePlayer _outactor)))
  (Sequencer|Player|Play _output_get :!class /Script/MovieScene.MovieSceneSequencePlayer)
  (Audio|PlaySoundatLocation "/Game/Astronaut/Sound/SE_InitSeq.SE_InitSeq" (Transformation|GetActorLocation) "0, 0, 0" 1.0 1.0 0.0 0 0 0)
  (Utilities|FlowControl|Delay 7.0)
  (Sequencer|Player|Pause _output_get)
  (Class|AstronautCharacter|OpenInfoWidget (Utilities|Name|MakeLiteralName "Trigger")))

(event EventOpenInfoWidget
  (params (Key :type Name%20%28by%20ref%29 :default "None"))
  (bind _infowidget (Variables|Default|GetInfoWidget))
  (Development|SetHiddeninGame _infowidget false false)
  (Collision|SetCollisionEnabled _infowidget "QueryAndPhysics")
  (bind _returnvalue (UserInterface|CreateWidget (.Value (Utilities|Map|Find (Variables|Default|GetInfoWidgetMapper) Key))))
  (UserInterface|SetWidget _infowidget _returnvalue)
  (Class|InfoWidget|Activate _returnvalue))

(event EventCloseInfoWidget
  (params (Key :type Name%20%28by%20ref%29 :default "None"))
  (bind _asinfo_widget (Utilities|Casting|CastToInfoWidget (UserInterface|GetWidget (Variables|Default|GetInfoWidget)))
    (:then
      (Class|InfoWidget|Deactivate _asinfo_widget)
      (CallFunction|HideInfoWidget))
    (:CastFailed
      _))
  (switch name Key
    (:Trigger
      (Utilities|FlowControl|Delay 1.0)
      (Class|AstronautCharacter|OpenSelectMissionPanel))
    (:Snapturn
      (Utilities|FlowControl|Delay 1.0)
      (Variables|Default|SetbMovable true)
      (Class|AstronautCharacter|OpenInfoWidget (Utilities|Name|MakeLiteralName "Move")))
    (:IVA
      (Variables|Default|SetbMovable true))
    (:Hook
      (Utilities|FlowControl|Delay 1.0)
      (Class|AstronautCharacter|OpenInfoWidget (Utilities|Name|MakeLiteralName "EVA")))
    (:EVA
      (Variables|Default|SetbMovable true))))

(event EventPlayCrossFade
  (bind _outactor (Sequencer|Player|CreateLevelSequencePlayer "/Game/Asset/Common/Sequence/SQ_CrossFade.SQ_CrossFade"))
  (Sequencer|Player|Play (Variables|/Script/LevelSequence.LevelSequenceActor|GetSequencePlayer _outactor) :!class /Script/MovieScene.MovieSceneSequencePlayer))

(event EventPlayMissionInitSequence
  (Utilities|FlowControl|Delay 1.0)
  (Sequencer|Player|Play (Variables|Default|GetInitialSequenceRef) :!class /Script/MovieScene.MovieSceneSequencePlayer)
  (Utilities|FlowControl|Delay 2.0)
  (Class|AstronautCharacter|InitializeMission))

(event Input|ActionEvents|InputActionTest
  (params (Key :type Key%20Structure :default "None"))
  (:Pressed
    (Class|AstronautCharacter|CloseInfoWidget (Utilities|Name|MakeLiteralName "Trigger"))))

(event Input|ActionEvents|InputActionTest2
  (params (Key :type Key%20Structure :default "None"))
  (:Pressed
    (Class|AstronautCharacter|SelectMission (Math|Conversions|ToInteger(Byte) (Utilities|Enum|LiteralenumEAstronautMissionType "CSM")))))

(event Input|ActionEvents|InputActionTest3
  (params (Key :type Key%20Structure :default "None"))
  (:Pressed
    (Class|AstronautCharacter|SelectMission (Math|Conversions|ToInteger(Byte) (Utilities|Enum|LiteralenumEAstronautMissionType "LEM")))))

(fn ConstructionScript)