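; BP_JudgeGameMode is the game mode for the judge courtroom level, sequencing narrated captions across the trial's phases.
; On BeginPlay it caches the prosecutor and lawyer actors, then after a short delay shows the entry caption, whose end toggles player movement and shows a guide caption.
; It binds StartOfTrial and StartOfCourtBattle events to further captions; the battle event also plays both NPCs' sit-to-stand animations and reveals their script widgets.
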(event Custom|StartOfCourtBattle_Event_0
  (bind _prosecutor (Variables|Default|GetProsecutor))
  (bind _lawyer (Variables|Default|GetLawyer))
  (CallFunction|CreateCaption (Variables|Default|GetNStartOfCourtBattleScript) (Variables|Default|GetNStartOfCourtBattleDelay) (Game|GetPlayerController 0))
  (Utilities|FlowControl|Sequence
    (:then_0
      (Components|Animation|PlayAnimation (Variables|/Script/Engine.Character|GetMesh _prosecutor) "/Game/Asset/Judge/ActorCore_Sample_Motions/Pose_dance_catwalk_Female/NPC_Male_sit_to_Stand_Anim.NPC_Male_sit_to_Stand_Anim" false)
      (Development|SetHiddeninGame (Variables|/Game/Asset/Common/CitizenNPC/Character/Blueprints/BP_Character.BP_Character_C|GetScriptWidget _prosecutor) false false))
    (:then_1
      (Components|Animation|PlayAnimation (Variables|/Script/Engine.Character|GetMesh _lawyer) "/Game/Asset/Judge/ActorCore_Sample_Motions/Idle_walk_sit_Female_Motion/NPC_Female_sit_to_Stand_Anim.NPC_Female_sit_to_Stand_Anim" false)
      (Development|SetHiddeninGame (Variables|/Game/Asset/Common/CitizenNPC/Character/Blueprints/BP_Character.BP_Character_C|GetScriptWidget _lawyer) false false))))

(event Custom|StartOfTrial_Event_0
  (CallFunction|CreateCaption (Variables|Default|GetNTrialBeginsScript) (Variables|Default|GetNTrialBeginsDelay) (Game|GetPlayerController 0)))

(event Custom|CaptionEnd_Event_0
  (Components|Activation|ToggleActive (Variables|/Script/Engine.Character|GetCharacterMovement (Game|GetPlayerCharacter 0)))
  (CallFunction|CreateCaption (Variables|Default|GetNGuideScript) (Variables|Default|GetNGuideDelay) (Game|GetPlayerController 0)))

(event EventBeginPlay
  (Utilities|FlowControl|Sequence
    (:then_0
      (bind _returnvalue (Actor|GetActorOfClass "/Game/Judge/Character/NPC/BP_Prosecutor.BP_Prosecutor_C"))
      (Variables|Default|SetProsecutor _returnvalue)
      (bind _returnvalue_2 (Actor|GetActorOfClass "/Game/Judge/Character/NPC/BP_Lawyer.BP_Lawyer_C"))
      (Variables|Default|SetLawyer _returnvalue_2))
    (:then_1
      (Utilities|FlowControl|Delay 2.0)
      (bind _widget (CallFunction|CreateCaption (Variables|Default|GetNEnterScript) (Variables|Default|GetNEnterDelay) (Game|GetPlayerController 0)))
      (EventDispatchers|AssignCaptionEnd _widget (delegate Custom|CaptionEnd_Event_0))
      (EventDispatchers|AssignStartOfTrial (delegate Custom|StartOfTrial_Event_0))
      (EventDispatchers|AssignStartOfCourtBattle (delegate Custom|StartOfCourtBattle_Event_0)))))

(fn ConstructionScript)