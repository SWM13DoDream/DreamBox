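; Lawyer NPC Blueprint that prepares the lawyer's script for the judge game.
; On BeginPlay, after the parent logic, it runs four steps in sequence: motive, defendant thoughts, reimbursement and final opinion.
; Each step passes its DataTable to AddArray along with that section's script and delay variables.
; EnableWidget and DisableWidget events show and hide the ScriptWidget.
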(event EventBeginPlay
  (|CallParentFunction)
  ;[0.9753 1 0.413] Lawyer Script Logic
  (Utilities|FlowControl|Sequence
    (:then_0
      (|MotiveScript))
    (:then_1
      (|DefendantThoughtsScript))
    (:then_2
      (|ReimbursementScript))
    (:then_3
      (|FinalOpinionScript))))

(event EventDisableWidget
  ;[1 0.3991 0.3294] Widget Enable & Disable
  (Rendering|SetVisibility (Variables|Default|GetScriptWidget) false false))

(event EventEnableWidget
  ;[1 0.3991 0.3294] Widget Enable & Disable
  (Rendering|SetVisibility (Variables|Default|GetScriptWidget) true false))

(fn ConstructionScript
  (|CallParentFunction))