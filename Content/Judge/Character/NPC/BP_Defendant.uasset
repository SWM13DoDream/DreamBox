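; BP_Defendant is the defendant NPC in a courtroom judge game, set up to deliver a final opinion script.
; On BeginPlay it runs the parent logic, then FinalOpinionScript, which passes the FinalOpinion data table, script and delay variables to AddArray.
; EnableWidget and DisableWidget events show and hide its ScriptWidget.
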(event EventBeginPlay
  (|CallParentFunction)
  ;[0.9753 1 0.413] Defendant Script Logic
  (|FinalOpinionScript))

(event EventDisableWidget
  ;[1 0.3991 0.3294] Widget Enable & Disable
  (Rendering|SetVisibility (Variables|Default|GetScriptWidget) false false))

(event EventEnableWidget
  ;[1 0.3991 0.3294] Widget Enable & Disable
  (Rendering|SetVisibility (Variables|Default|GetScriptWidget) true false))

(fn ConstructionScript
  (|CallParentFunction))