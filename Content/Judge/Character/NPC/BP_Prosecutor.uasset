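; BP_Prosecutor is a prosecutor NPC for the Judge game that holds the prosecutor's scripted statements.
; On BeginPlay, after the parent's logic, AddArray is called on four DataTables with matching script and delay arrays: criminal background, criminal record, degree of damage and final opinion.
; EnableWidget and DisableWidget events show and hide its ScriptWidget.
; Overlap and Tick are disabled, and playback of the lines is not handled here.
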(event EventBeginPlay
  (|CallParentFunction)
  (Utilities|FlowControl|Sequence
    (:then_0
      (CallFunction|AddArray (Variables|DataTable|GetCriminalBackground) (Variables|Script|GetCriminalBackgroundScript) (Variables|Delay|GetCriminalBackgroundDelay)))
    (:then_1
      (CallFunction|AddArray (Variables|DataTable|GetCriminalRecord) (Variables|스크립트|GetCriminalRecordScript) (Variables|딜레이|GetCriminalRecordDelay)))
    (:then_2
      (CallFunction|AddArray (Variables|데이터테이블|GetDegreeOfDamage) (Variables|스크립트|GetDegreeOfDamageScript) (Variables|딜레이|GetDegreeOfDamageDelay)))
    (:then_3
      (CallFunction|AddArray (Variables|데이터테이블|GetFinalOpinion) (Variables|스크립트|GetFinalOpinionScript) (Variables|딜레이|GetFinalOpinionDelay)))))

(event Collision|EventActorBeginOverlap
  (params (OtherActor :type Actor%20Object%20Reference)))

(event EventTick
  (params (DeltaSeconds :type Float%20%28single-precision%29))
  (|CallParentFunction DeltaSeconds) ; This node is disabled and will not be called.\nDrag off pins to build functionality.
)

(event EventDisableWidget
  (Rendering|SetVisibility (Variables|Default|GetScriptWidget) false false))

(event EventEnableWidget
  (Rendering|SetVisibility (Variables|Default|GetScriptWidget) true false))

(fn ConstructionScript
  (|CallParentFunction))