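; VR player character that spawns left and right BP_MotionController3DWidget actors, whose widget interaction turns trigger presses into left-mouse clicks on 3D UI.
; BeginPlay sets floor tracking for SteamVR or Oculus, toggles CharacterMovement's active state and shows a fade-in widget.
; Left-hand axis input moves the character relative to camera facing on the horizontal plane.
; A DoOnce-gated, non-looping timer plays a delayed footstep during movement, and landing plays one too.
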(event Custom|PlayFootSound
  (Audio|PlaySoundatLocation 0 (- (Transformation|GetActorLocation) "0, 0,44.000000") "0, 0, 0" 1.0 1.0 0.0 0 0 0))

(event EventOnMovementModeChanged
  (params (PrevMovementMode :type EMovementMode%20Enum :default "MOVE_None") (NewMovementMode :type EMovementMode%20Enum :default "MOVE_None") (PrevCustomMode :type Byte :default 0) (NewCustomMode :type Byte :default 0))
  (if (and (Utilities|Enum|Equal(Enum) PrevMovementMode "MOVE_Falling") (Utilities|Enum|Equal(Enum) NewMovementMode "MOVE_Walking"))
    (CallFunction|PlayFootSound)))

(event EventBeginPlay
  (bind _returnvalue (Math|Transform|MakeTransform "0, 0, 0"))
  (Utilities|FlowControl|Sequence
    (:then_0
      (switch name (Class|HeadMountedDisplayFunctionLibrary|GetHMDDeviceName)
        (:SteamVR
          _)
        (:OculusHMD
          _))
      (Class|HeadMountedDisplayFunctionLibrary|SetTrackingOrigin "Floor"))
    (:then_1
      (Utilities|FlowControl|Sequence
        (:then_0
          (bind _returnvalue_2 (Game|SpawnActorfromClass "/Game/Asset/Common/VRContentExamples/UI/3DWidget/BP_MotionController3DWidget.BP_MotionController3DWidget_C" _returnvalue "AlwaysSpawn" self "Left" 0))
          (bind _output_get (Variables|Default|SetLeftController _returnvalue_2))
          (Transformation|AttachComponentToComponent _output_get (Variables|Transformation|GetRootComponent) "None" "SnapToTarget" "SnapToTarget" "KeepWorld" false))
        (:then_1
          (bind _returnvalue_3 (Game|SpawnActorfromClass "/Game/Asset/Common/VRContentExamples/UI/3DWidget/BP_MotionController3DWidget.BP_MotionController3DWidget_C" _returnvalue "AlwaysSpawn" self "Right" 0))
          (bind _output_get_2 (Variables|Default|SetRightController _returnvalue_3))
          (Transformation|AttachComponentToComponent _output_get_2 (Variables|Transformation|GetRootComponent) "None" "SnapToTarget" "SnapToTarget" "KeepWorld" false))))
    (:then_2
      (Input|SetInputModeGameOnly (Game|GetPlayerController 0))
      (Components|Activation|ToggleActive (Variables|Character|GetCharacterMovement))
      (CallFunction|FadeinEffect))))

(event Input|ActionEvents|InputActionLeftTrigger
  (params (Key :type Key%20Structure))
  (bind _leftcontroller (Variables|Default|GetLeftController))
  (bind _widgetinteraction (Variables|/Game/Asset/Common/VRContentExamples/UI/3DWidget/BP_MotionController3DWidget.BP_MotionController3DWidget_C|GetWidgetInteraction _leftcontroller))
  (:Pressed
    (Class|WidgetInteractionComponent|PressPointerKey _widgetinteraction "LeftMouseButton"))
  (:Released
    (Class|WidgetInteractionComponent|ReleasePointerKey _widgetinteraction "LeftMouseButton")))

(event Input|ActionEvents|InputActionRightTrigger
  (params (Key :type Key%20Structure))
  (bind _rightcontroller (Variables|Default|GetRightController))
  (bind _widgetinteraction (Variables|/Game/Asset/Common/VRContentExamples/UI/3DWidget/BP_MotionController3DWidget.BP_MotionController3DWidget_C|GetWidgetInteraction _rightcontroller))
  (:Pressed
    (Class|WidgetInteractionComponent|PressPointerKey _widgetinteraction "LeftMouseButton"))
  (:Released
    (Class|WidgetInteractionComponent|ReleasePointerKey _widgetinteraction "LeftMouseButton")))

(event Input|AxisEvents|InputAxisMovementAxisLeft_X
  (params (AxisValue :type Float%20%28single-precision%29))
  (bind _returnvalue (Transformation|GetVelocity))
  (bind _camera (Variables|Default|GetCamera))
  (bind _returnvalue_2 (Math|Vector|GetRightVector _camera))
  (if (not (== AxisValue 0.0))
    (Pawn|Input|AddMovementInput (Math|Vector|MakeVector (.x _returnvalue_2) (.y _returnvalue_2) 0.0) (* AxisValue (Variables|Default|GetMovementSpeed)) false)
    (if (and (Math|Boolean|ORBoolean (> (.x _returnvalue) 2.0) (< (.x _returnvalue) -2.0) (> (.y _returnvalue) 2.0) (< (.y _returnvalue) -2.0)) (== (.z _returnvalue) 0.0))
      (Utilities|FlowControl|DoOnce false :!label _label
        (:Completed
          (bind _returnvalue_3 (Utilities|Time|SetTimerbyEvent (delegate Custom|PlayFootSound) (Variables|Default|GetFootStepInterval)))))
      (else
        (Utilities|Time|ClearandInvalidateTimerbyHandle _returnvalue_3)
        (goto _label Reset)))))

(event Input|AxisEvents|InputAxisMovementAxisLeft_Y
  (params (AxisValue :type Float%20%28single-precision%29))
  (bind _returnvalue (Transformation|GetVelocity))
  (bind _camera (Variables|Default|GetCamera))
  (bind _returnvalue_2 (Math|Vector|GetForwardVector _camera))
  (if (not (== AxisValue 0.0))
    (Pawn|Input|AddMovementInput (Math|Vector|MakeVector (.x _returnvalue_2) (.y _returnvalue_2) 0.0) (* AxisValue (Variables|Default|GetMovementSpeed)) false)
    (if (and (Math|Boolean|ORBoolean (> (.x _returnvalue) 2.0) (< (.x _returnvalue) -2.0) (> (.y _returnvalue) 2.0) (< (.y _returnvalue) -2.0)) (== (.z _returnvalue) 0.0))
      (Utilities|FlowControl|DoOnce false :!label _label
        (:Completed
          (bind _returnvalue_3 (Utilities|Time|SetTimerbyEvent (delegate Custom|PlayFootSound) (Variables|Default|GetFootStepInterval)))))
      (else
        (Utilities|Time|ClearandInvalidateTimerbyHandle _returnvalue_3)
        (goto _label Reset)))))

(fn ConstructionScript)

(fn FadeinEffect
  (bind _returnvalue (UserInterface|CreateWidget "/Game/Judge/UI/FadeEffect/WI_Fade.WI_Fade_C" (Game|GetPlayerController 0)))
  (UserInterface|Viewport|AddtoViewport _returnvalue 0)
  (Default|Fadein _returnvalue))