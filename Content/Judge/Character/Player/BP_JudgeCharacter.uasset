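; BP_JudgeCharacter is the player character for the Judge game mode, with an intro sequence that is currently not wired to any event.
; The unconnected chain toggles movement, plays a WI_Fade fade-in through FadeEffect, waits briefly, then creates a caption from the game mode's NEnter script and delay.
; A CaptionEndEvent bound to that caption toggles movement again when it ends.
; BeginPlay and the construction script are empty.
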(event Custom|Caption%20End%20Event
  (Components|Activation|ToggleActive (Variables|Character|GetCharacterMovement)))

(event EventBeginPlay)

(fn ConstructionScript)

(fn FadeEffect
  (bind _returnvalue (UserInterface|CreateWidget "/Game/Judge/UI/FadeEffect/WI_Fade.WI_Fade_C"))
  (UserInterface|Viewport|AddtoViewport _returnvalue 0)
  (Default|Fadein _returnvalue))