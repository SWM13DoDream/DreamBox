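; BP_JudgeCharacter is the character Blueprint for the Judge part of the game, with helpers for a screen fade and scripted captions.
; FadeEffect shows a fade-in widget, and CreateCaption adds a caption widget fed a script and delay.
; An unconnected intro sequence would toggle movement, fade in, play the game mode's entry caption, then toggle movement again through CaptionEndEvent.
; BeginPlay is empty, so that intro never runs.
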(event Custom|Caption%20End%20Event
  (Components|Activation|ToggleActive (Variables|Character|GetCharacterMovement)))

(event EventBeginPlay)

(fn ConstructionScript)

(fn CreateCaption
  (params (Script :type Array%20of%20Strings) (Delay :type Array%20of%20Floats%20%28single-precision%29))
  (bind _returnvalue (UserInterface|CreateWidget "/Game/Judge/UI/Caption/WI_Caption.WI_Caption_C"))
  (Variables|/Game/Judge/UI/Caption/WI_Caption.WI_Caption_C|SetPlayScript _returnvalue Script)
  (Variables|/Game/Judge/UI/Caption/WI_Caption.WI_Caption_C|SetPlayDelay _returnvalue Delay)
  (UserInterface|Viewport|AddtoViewport _returnvalue 0)
  (return _returnvalue))

(fn FadeEffect
  (bind _returnvalue (UserInterface|CreateWidget "/Game/Judge/UI/FadeEffect/WI_Fade.WI_Fade_C"))
  (UserInterface|Viewport|AddtoViewport _returnvalue 0)
  (Default|Fadein _returnvalue))