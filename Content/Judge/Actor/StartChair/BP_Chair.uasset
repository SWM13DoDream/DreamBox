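; BP_Chair is the judge's start chair, an actor that begins the trial when the judge character walks into its trigger.
; On overlap it destroys the trigger so it fires once, then plays a WI_Fade widget fade-out.
; After a delay it moves the character to the Arrow component's transform, fades back in and tells BP_JudgeGameMode to start the trial.
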(event OnComponentBeginOverlap(Trigger)
  (params (OverlappedComponent :type Primitive%20Component%20Object%20Reference) (OtherActor :type Actor%20Object%20Reference) (OtherComp :type Primitive%20Component%20Object%20Reference) (OtherBodyIndex :type Integer) (bFromSweep :type Boolean) (SweepResult :type Hit%20Result%20Structure%20%28by%20ref%29))
  (bind _arrow (Variables|Default|GetArrow))
  (bind _asbp_judge_character (Utilities|Casting|CastToBP_JudgeCharacter OtherActor))
  (Components|DestroyComponent OverlappedComponent)
  (bind _returnvalue (UserInterface|CreateWidget "/Game/Judge/UI/FadeEffect/WI_Fade.WI_Fade_C" (Game|GetPlayerController 0)))
  (UserInterface|Viewport|AddtoViewport _returnvalue 0)
  (Default|FadeOut _returnvalue)
  (Utilities|FlowControl|Delay 2.0)
  (Transformation|SetActorLocationAndRotation _asbp_judge_character (Transformation|GetWorldLocation _arrow) (Transformation|GetWorldRotation _arrow))
  (Default|Fadein _returnvalue)
  (Utilities|FlowControl|Delay 1.5)
  (Default|CallStartOfTrial (.AsBP%20Judge%20Game%20Mode (Utilities|Casting|CastToBP_JudgeGameMode (Game|GetGameMode))))
  (Development|PrintString "Hello"))

(fn ConstructionScript)