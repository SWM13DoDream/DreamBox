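; BP_FloatPetitionWidget is an actor that presents the WI_Petition widget through its Widget component.
; On BeginPlay it binds to the petition's Close event and sets the WidgetIsActive flag on JudgeGameMode.
; When Close fires, it destroys every valid actor implementing the FloatingWidget interface, not only a specific instance, then clears the flag.
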(event Custom|Close_Event_0
  (bind _outactors (Actor|GetAllActorswithInterface "/Game/Judge/Actor/Introduce/FloatingWidget.FloatingWidget_C"))
  (for _array_element _outactors
    (Utilities|IsValid _array_element
      (:Is%20Valid
        (Actor|DestroyActor _array_element))))
  (Variables|/Script/DreamBox.JudgeGameMode|SetbWidgetIsActive (.AsJudge%20Game%20Mode (Utilities|Casting|CastToJudgeGameMode (Game|GetGameMode))) false))

(event EventBeginPlay
  (EventDispatchers|AssignClose (.AsWI%20Petition (Utilities|Casting|CastToWI_Petition (UserInterface|GetWidget (Variables|Default|GetWidget)))) (delegate Custom|Close_Event_0))
  (Variables|/Script/DreamBox.JudgeGameMode|SetbWidgetIsActive (.AsJudge%20Game%20Mode (Utilities|Casting|CastToJudgeGameMode (Game|GetGameMode))) true))

(fn ConstructionScript)