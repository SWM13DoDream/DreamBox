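; BP_FloatOverviewWidget is an actor that hosts the WI_Overview widget in the Judge game's introduction.
; On BeginPlay it sets the WidgetIsActive and Overview flags on JudgeGameMode and binds to the widget's Close dispatcher.
; When the widget closes, it calls RemoveWidget, then asks JudgeGameMode whether the court battle can start and triggers StartOfCourtBattle if so.
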(event Custom|Close_Event_0
  (bind _returnvalue (Game|GetGameMode))
  (bind _asjudge_game_mode (Utilities|Casting|CastToJudgeGameMode _returnvalue))
  (CallFunction|RemoveWidget)
  (bind _returnvalue_2 (Class|JudgeGameMode|TryStartOfCourtBattle _asjudge_game_mode))
  (if _returnvalue_2
    (Default|CallStartOfCourtBattle _asjudge_game_mode)))

(event EventBeginPlay
  (bind _returnvalue (Game|GetGameMode))
  (bind _asjudge_game_mode (Utilities|Casting|CastToJudgeGameMode _returnvalue))
  (Variables|/Script/DreamBox.JudgeGameMode|SetbWidgetIsActive _asjudge_game_mode true)
  (Variables|/Script/DreamBox.JudgeGameMode|SetbOverview _asjudge_game_mode true)
  (EventDispatchers|AssignClose (.AsWI%20Overview (Utilities|Casting|CastToWI_Overview (UserInterface|GetWidget (Variables|Default|GetWidget)))) (delegate Custom|Close_Event_0)))

(fn ConstructionScript)