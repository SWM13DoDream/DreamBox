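; Floating widget actor that shows the condition introduction in the Judge game mode and gates the start of the court battle.
; On BeginPlay it binds to the WI_Condition widget's close event and flags the game mode as having an active widget.
; On close it sets the Condition flag, destroys every actor implementing FloatingWidget, clears the active flag and calls TryStartOfCourtBattle.
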(event Custom|Close_Event_0
  (bind _returnvalue (Game|GetGameMode))
  (bind _asjudge_game_mode (Utilities|Casting|CastToJudgeGameMode _returnvalue))
  (Variables|/Script/DreamBox.JudgeGameMode|SetbCondition _asjudge_game_mode true)
  (bind _outactors (Actor|GetAllActorswithInterface "/Game/Judge/Actor/Introduce/FloatingWidget.FloatingWidget_C"))
  (for _array_element _outactors
    (Actor|DestroyActor _array_element))
  (Variables|/Script/DreamBox.JudgeGameMode|SetbWidgetIsActive _asjudge_game_mode false)
  (Class|JudgeGameMode|TryStartOfCourtBattle _asjudge_game_mode))

(event EventBeginPlay
  (EventDispatchers|AssignClose (.AsWI%20Condition (Utilities|Casting|CastToWI_Condition (UserInterface|GetWidget (Variables|Default|GetWidget)))) (delegate Custom|Close_Event_0))
  (Variables|/Script/DreamBox.JudgeGameMode|SetbWidgetIsActive (.AsJudge%20Game%20Mode (Utilities|Casting|CastToJudgeGameMode (Game|GetGameMode))) true))

(fn ConstructionScript)