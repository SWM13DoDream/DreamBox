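; BP_FloatMerchantPetitionWidget is a floating widget actor that presents the merchant petition in the Judge game.
; On BeginPlay it binds to the W_MerchantPetition close event and sets the WidgetIsActive and MPetition flags on JudgeGameMode.
; Closing the petition removes the widget, then asks the game mode whether final judgement can start and triggers it if so.
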(event Custom|Close_Event_0
  (bind _returnvalue (Game|GetGameMode))
  (bind _asjudge_game_mode (Utilities|Casting|CastToJudgeGameMode _returnvalue))
  (CallFunction|CallRemoveFloatWidget)
  (bind _returnvalue_2 (Class|JudgeGameMode|TryStartOfFinalJudgement _asjudge_game_mode))
  (if _returnvalue_2
    (Default|CallStartOfFinalJudgement _asjudge_game_mode)))

(event EventBeginPlay
  (bind _returnvalue (Game|GetGameMode))
  (bind _asjudge_game_mode (Utilities|Casting|CastToJudgeGameMode _returnvalue))
  (EventDispatchers|BindEventtoClose (.AsWI%20Merchant%20Petition (Utilities|Casting|CastToW_MerchantPetition (UserInterface|GetWidget (Variables|Default|GetWidget)))) (delegate Custom|Close_Event_0))
  (Variables|/Script/DreamBox.JudgeGameMode|SetbWidgetIsActive _asjudge_game_mode true)
  (Variables|/Script/DreamBox.JudgeGameMode|SetbMPetition _asjudge_game_mode true))

(event EventCallRemoveFloatWidget
  (CallFunction|RemoveWidget))

(fn ConstructionScript)