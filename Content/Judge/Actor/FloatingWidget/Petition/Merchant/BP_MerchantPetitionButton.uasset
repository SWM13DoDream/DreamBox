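; BP_MerchantPetitionButton is an actor that presents a merchant petition button as floating widgets with a name label.
; On BeginPlay it writes its Name variable into the W_FloatName label held by NameWidget.
; It also binds hover and unhover events on the W_MerchantPetitionButton in ButtonWidget, which play the name label's animation forward or back through Animate.
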(event Custom|HoverEvent_Event_0
  (Default|Animate (.AsW%20Float%20Name (Utilities|Casting|CastToW_FloatName (UserInterface|GetWidget (Variables|Default|GetNameWidget)))) true))

(event Custom|UnHoverEvent_Event_0
  (Default|Animate (.AsW%20Float%20Name (Utilities|Casting|CastToW_FloatName (UserInterface|GetWidget (Variables|Default|GetNameWidget)))) false))

(event EventBeginPlay
  (bind _buttonwidget (Variables|Default|GetButtonWidget))
  (bind _returnvalue (UserInterface|GetWidget _buttonwidget))
  (bind _asw_merchant_petition_button (Utilities|Casting|CastToW_MerchantPetitionButton _returnvalue))
  (Utilities|FlowControl|Sequence
    (:then_0
      (Rendering|Components|TextRender|SetText (Variables|/Game/Judge/UI/FloatWidget/W_FloatName.W_FloatName_C|GetNameBox (.AsW%20Float%20Name (Utilities|Casting|CastToW_FloatName (UserInterface|GetWidget (Variables|Default|GetNameWidget))))) (Variables|Default|GetName)))
    (:then_1
      (EventDispatchers|AssignHoverEvent _asw_merchant_petition_button (delegate Custom|HoverEvent_Event_0))
      (EventDispatchers|AssignUnHoverEvent _asw_merchant_petition_button (delegate Custom|UnHoverEvent_Event_0)))))

(fn ConstructionScript)