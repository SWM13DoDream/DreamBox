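; Floating widget actor that presents the friend petition during the Judge game.
; On BeginPlay it binds to the WI_FriendPetition widget's close event and sets the JudgeGameMode's WidgetIsActive and FPetition flags.
; When the widget closes, it removes itself and asks the game mode whether final judgement can start, triggering it if so.
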(event Custom|Close_Event_0
  (bind _returnvalue (Game|GetGameMode))
  (bind _asjudge_game_mode (Utilities|Casting|CastToJudgeGameMode _returnvalue))
  (CallFunction|CallRemoveFloatWidget)
  (bind _returnvalue_2 (Class|JudgeGameMode|TryStartOfFinalJudgement _asjudge_game_mode))
  (if _returnvalue_2
    (Default|CallStartOfFinalJudgement _asjudge_game_mode)))

(event EventBeginPlay
  (bind _returnvalue (Game|GetGameMode))
  (bind _asjudge_game_mode (Utilities|Casting|CastToJudgeGameMode _returnvalue))
  (EventDispatchers|BindEventtoClose (.AsWI%20Friend%20Petition (Utilities|Casting|CastToWI_FriendPetition (UserInterface|GetWidget (Variables|Default|GetWidget)))) (delegate Custom|Close_Event_0))
  (Variables|/Script/DreamBox.JudgeGameMode|SetbWidgetIsActive _asjudge_game_mode true)
  (Variables|/Script/DreamBox.JudgeGameMode|SetbFPetition _asjudge_game_mode true))

(event EventCallRemoveFloatWidget
  (CallFunction|RemoveWidget))

(fn ConstructionScript)