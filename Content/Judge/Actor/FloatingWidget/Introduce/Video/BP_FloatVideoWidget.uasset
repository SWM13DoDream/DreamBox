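; BP_FloatVideoWidget is a floating widget that presents a W_Video screen, apparently as part of the introduction before a court battle.
; On BeginPlay it binds to the video widget's Close event and flags the JudgeGameMode that a widget and video are active.
; On close it removes the widget, then calls StartOfCourtBattle on the game mode if TryStartOfCourtBattle succeeds.
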(event Custom|Close_Event_0
  (bind _returnvalue (Game|GetGameMode))
  (bind _asjudge_game_mode (Utilities|Casting|CastToJudgeGameMode _returnvalue))
  (CallFunction|CallRemoveFloatWidget)
  (bind _returnvalue_2 (Class|JudgeGameMode|TryStartOfCourtBattle _asjudge_game_mode))
  (if _returnvalue_2
    (Default|CallStartOfCourtBattle _asjudge_game_mode)))

(event EventBeginPlay
  (bind _returnvalue (Game|GetGameMode))
  (bind _asjudge_game_mode (Utilities|Casting|CastToJudgeGameMode _returnvalue))
  (EventDispatchers|AssignClose (.AsWI%20Video (Utilities|Casting|CastToW_Video (UserInterface|GetWidget (Variables|Default|GetWidget)))) (delegate Custom|Close_Event_0))
  (Variables|/Script/DreamBox.JudgeGameMode|SetbWidgetIsActive _asjudge_game_mode true)
  (Variables|/Script/DreamBox.JudgeGameMode|SetbVideo _asjudge_game_mode true))

(event EventCallRemoveFloatWidget
  (CallFunction|RemoveWidget))

(fn ConstructionScript)