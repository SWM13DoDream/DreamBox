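; BP_FloatSignT is a floating sign actor that shows a title and description on a W_Sign widget in its Screen component.
; BeginPlay copies its TitleText and DescriptionText into the widget.
; Box overlaps by a VRCharacter drive the widget's Animate: entering plays it true only when Toggle is set, and leaving plays it false only when Toggle is unset.
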(event OnComponentEndOverlap(Box)
  (params (OverlappedComponent :type Primitive%20Component%20Object%20Reference) (OtherActor :type Actor%20Object%20Reference) (OtherComp :type Primitive%20Component%20Object%20Reference) (OtherBodyIndex :type Integer))
  (Utilities|Casting|CastToVRCharacter OtherActor)
  (if (not (Variables|Default|GetbToggle))
    (Default|Animate (.AsW%20Sign (Utilities|Casting|CastToW_Sign (UserInterface|GetWidget (Variables|Default|GetScreen)))) false)))

(event OnComponentBeginOverlap(Box)
  (params (OverlappedComponent :type Primitive%20Component%20Object%20Reference) (OtherActor :type Actor%20Object%20Reference) (OtherComp :type Primitive%20Component%20Object%20Reference) (OtherBodyIndex :type Integer) (bFromSweep :type Boolean) (SweepResult :type Hit%20Result%20Structure%20%28by%20ref%29))
  (Utilities|Casting|CastToVRCharacter OtherActor)
  (if (Variables|Default|GetbToggle)
    (Default|Animate (.AsW%20Sign (Utilities|Casting|CastToW_Sign (UserInterface|GetWidget (Variables|Default|GetScreen)))) true)))

(event EventBeginPlay
  (bind _screen (Variables|Default|GetScreen))
  (bind _returnvalue (UserInterface|GetWidget _screen))
  (bind _asw_sign (Utilities|Casting|CastToW_Sign _returnvalue))
  (Rendering|Components|TextRender|SetText (Variables|/Game/Judge/UI/Sign/W_Sign.W_Sign_C|GetTitleText _asw_sign) (Variables|Default|GetTitleText))
  (Rendering|Components|TextRender|SetText (Variables|/Game/Judge/UI/Sign/W_Sign.W_Sign_C|GetDescriptionText _asw_sign) (Variables|Default|GetDescriptionText)))

(fn ConstructionScript)