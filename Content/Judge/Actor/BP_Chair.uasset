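; BP_Chair is a trigger actor in the Judge game that starts the trial when BP_JudgeCharacter overlaps it.
; The overlap creates a WI_Fade widget, plays a fade-out, waits briefly, then plays a long fade-in.
; It then has the character show the trial-begins caption using script and delay from BP_JudgeGameMode, and calls CallTrialBegins on that game mode.
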(event Collision|EventActorBeginOverlap
  (params (OtherActor :type Actor%20Object%20Reference))
  (bind _returnvalue (Game|GetGameMode))
  (bind _asbp_judge_game_mode (Utilities|Casting|CastToBP_JudgeGameMode _returnvalue))
  (bind _asbp_judge_character (Utilities|Casting|CastToBP_JudgeCharacter OtherActor))
  (bind _returnvalue_2 (UserInterface|CreateWidget "/Game/Judge/UI/FadeEffect/WI_Fade.WI_Fade_C" (Game|GetPlayerController 0)))
  (UserInterface|Viewport|AddtoViewport _returnvalue_2 0)
  (Default|FadeOut _returnvalue_2)
  (Utilities|FlowControl|Delay 1.5)
  (Default|LongFadein _returnvalue_2)
  (Default|CreateCaption _asbp_judge_character (Variables|/Script/DreamBox.JudgeGameMode|GetN_TrialBeginsScript _asbp_judge_game_mode) (Variables|/Script/DreamBox.JudgeGameMode|GetN_TrialBeginsDelay _asbp_judge_game_mode))
  (Default|CallTrialBegins _asbp_judge_game_mode))

(fn ConstructionScript)