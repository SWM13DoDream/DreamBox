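; BP_TempCharacter is a temporary player character for the Firefighter game with basic movement, look and jump controls.
; Axis inputs move it along the FollowingCamera's forward and right vectors and turn the controller's pitch and yaw, and Space jumps.
; Holding the left mouse button shows a ChildActor component and releasing hides it, without propagating visibility to its children.
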(event EventBeginPlay)

(event Input|AxisEvents|InputAxisMoveForward
  (params (AxisValue :type Float%20%28single-precision%29))
  (Pawn|Input|AddMovementInput (Math|Vector|GetForwardVector (Transformation|GetWorldRotation (Variables|Default|GetFollowingCamera))) AxisValue false))

(event Input|AxisEvents|InputAxisMoveRight
  (params (AxisValue :type Float%20%28single-precision%29))
  (Pawn|Input|AddMovementInput (Math|Vector|GetRightVector (Transformation|GetWorldRotation (Variables|Default|GetFollowingCamera))) AxisValue false))

(event Input|AxisEvents|InputAxisLookUp
  (params (AxisValue :type Float%20%28single-precision%29))
  (Pawn|Input|AddControllerPitchInput AxisValue))

(event Input|AxisEvents|InputAxisTurn
  (params (AxisValue :type Float%20%28single-precision%29))
  (Pawn|Input|AddControllerYawInput AxisValue))

(event Input|KeyboardEvents|SpaceBar
  (params (Key :type Key%20Structure :default "None"))
  (:Pressed
    (Character|Jump)))

(event Input|MouseEvents|LeftMouseButton
  (params (Key :type Key%20Structure :default "None"))
  (bind _childactor (Variables|Default|GetChildActor))
  (:Pressed
    (Rendering|SetVisibility _childactor true false))
  (:Released
    (Rendering|SetVisibility _childactor false false)))

(fn ConstructionScript)