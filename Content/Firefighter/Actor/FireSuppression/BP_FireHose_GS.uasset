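; Grabbable fire hose actor for the firefighter game, driven by grab and drop events from its BPAC_GS_Core component.
; Grabbing sets the player character's hose grab state to the holding hand, hides the Sphere, and registers the hose with the character on the first grab only.
; Dropping clears the grab state, shows the Sphere and deactivates the WaterEmitter, which this Blueprint never activates itself.
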(event OnDrop(BPAC_GS_Core)
  ;[1 0.8834 0.401] Grab 상태 업데이트
  (Class|FirefighterCharacter|SetHoseGrabState (.AsFirefighter%20Character (Utilities|Casting|CastToFirefighterCharacter (Game|GetPlayerCharacter 0))) "E_NONE")
  (Components|Activation|Deactivate (Variables|Default|GetWaterEmitter))
  (Rendering|SetVisibility (Variables|Default|GetSphere) true false))

(event OnGrabAction(Boolean)(BPAC_GS_Core)
  (params (Target :type BPAC%20HAC%20GS%20Object%20Reference) (Hand :type E_Hand%20Enum :default "NewEnumerator0") (Key :type E_ControllerButtons_Boolean%20Enum :default "NewEnumerator0") (Value :type Boolean))
  (bind _returnvalue (Game|GetPlayerCharacter 0))
  (bind _asfirefighter_character (Utilities|Casting|CastToFirefighterCharacter _returnvalue))
  ;[1 0.8834 0.401] Grab 상태 업데이트
  (if Value
    (Utilities|IsValid _asfirefighter_character
      (:Is%20Valid
        (Class|FirefighterCharacter|SetHoseGrabState _asfirefighter_character (Utilities|Select :Index Hand :NewEnumerator0 "E_LEFT" :NewEnumerator1 "E_RIGHT"))
        (Rendering|SetVisibility (Variables|Default|GetSphere) false false)
        (Utilities|FlowControl|DoOnce false
          (:Completed
            (Class|FirefighterCharacter|SetFireHoseRef _asfirefighter_character self)))))))

(fn ConstructionScript)