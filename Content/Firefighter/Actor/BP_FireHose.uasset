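; Fire hose actor whose Niagara water particles deal damage to fire where they report their positions.
; On BeginPlay it registers itself as the emitter's callback object to receive exported particle data.
; Each particle position triggers a multicast, directly on authority or via server RPC from remotes, applying small, tight radial damage.
; RS_ApplyDamageToFire and MCApplyDamageToFire are empty stubs.
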(event Custom|RS_ApplyDamageToFire
  (params (Location :type Vector)))

(event Custom|MultiCastApplyDamageToFire
  (params (Location :type Vector))
  (Game|Damage|ApplyRadialDamage 0.05 Location 5.0 0 0 self 0 false "ECC_Visibility"))

(event Custom|ServerRPCApplyDamageToFire
  (params (Location :type Vector))
  (CallFunction|MultiCastApplyDamagetoFire Location))

(event EventParticleData
  (params (Data :type Array%20of%20Basic%20Particle%20Data%20Structures) (NiagaraSystem :type Niagara%20System%20Object%20Reference))
  (for _array_element Data
    (Networking|SwitchHasAuthority
      (:Authority
        (CallFunction|MultiCastApplyDamagetoFire (.Position (Utilities|Struct|BreakBasicParticleData _array_element))))
      (:Remote
        (CallFunction|ServerRPCApplyDamagetoFire (.Position (Utilities|Struct|BreakBasicParticleData _array_element)))))))

(event EventBeginPlay
  (Niagara|SetNiagaraVariable(Object) (Variables|Default|GetWaterEmitter) "User.BP_Callback" self))

(fn ConstructionScript)

(fn MCApplyDamagetoFire
  (params (Location1 :type Vector)))