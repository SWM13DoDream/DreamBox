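; BP_GuideTrigger is a trigger actor that shows a fire suppression control guide widget when a player-tagged actor enters its volume.
; On begin overlap, a macro gates the guide on the referenced fire being valid and not yet suppressed, then the widget is made visible and plays its animation forward.
; End overlap calls the same animation with false, without checking the fire or changing visibility.
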(event OnComponentBeginOverlap(WidgetTrigger)
  (params (OverlappedComponent :type Primitive%20Component%20Object%20Reference) (OtherActor :type Actor%20Object%20Reference) (OtherComp :type Primitive%20Component%20Object%20Reference) (OtherBodyIndex :type Integer) (bFromSweep :type Boolean) (SweepResult :type Hit%20Result%20Structure%20%28by%20ref%29))
  (bind _widget (Variables|Default|GetWidget))
  (if (Actor|ActorHasTag OtherActor "Player")
    (|CheckFireIsValidAndSuppressed)
    (bind _asw_control_guide_fire_suppression (Utilities|Casting|CastToW_ControlGuide_FireSuppression (UserInterface|GetWidget _widget)))
    (Rendering|SetVisibility _widget true false)
    (Default|PlayAnim _asw_control_guide_fire_suppression true)))

(event OnComponentEndOverlap(WidgetTrigger)
  (params (OverlappedComponent :type Primitive%20Component%20Object%20Reference) (OtherActor :type Actor%20Object%20Reference) (OtherComp :type Primitive%20Component%20Object%20Reference) (OtherBodyIndex :type Integer))
  (if (Actor|ActorHasTag OtherActor "Player")
    (bind _asw_control_guide_fire_suppression (Utilities|Casting|CastToW_ControlGuide_FireSuppression (UserInterface|GetWidget (Variables|Default|GetWidget))))
    (Default|PlayAnim _asw_control_guide_fire_suppression false)))

(fn ConstructionScript)