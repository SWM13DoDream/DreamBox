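; BP_CauseOfFire is a fire investigation actor that shows an info text widget when the player comes near.
; BeginPlay caches the W_InvestigationInfo from its WidgetComponent and sets its InfoText.
; While the actor is activated, a Player-tagged actor entering InteractionTrigger makes the widget visible, refreshes the text and plays its animation.
; Leaving the trigger calls the animation with false, without hiding the component.
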(event OnComponentBeginOverlap(InteractionTrigger)
  (params (OverlappedComponent :type Primitive%20Component%20Object%20Reference) (OtherActor :type Actor%20Object%20Reference) (OtherComp :type Primitive%20Component%20Object%20Reference) (OtherBodyIndex :type Integer) (bFromSweep :type Boolean) (SweepResult :type Hit%20Result%20Structure%20%28by%20ref%29))
  (if (and (Actor|ActorHasTag OtherActor "Player") (Class|CauseOfFire|GetIsActivated))
    (Default|PlayAnim (Variables|Default|GetWidgetRef) true)
    (Rendering|SetVisibility (Variables|Default|GetWidgetComponent) true false)
    (Default|SetInfoText (Variables|Default|GetWidgetRef) (Variables|Gameplay|GetInfoText))))

(event OnComponentEndOverlap(InteractionTrigger)
  (params (OverlappedComponent :type Primitive%20Component%20Object%20Reference) (OtherActor :type Actor%20Object%20Reference) (OtherComp :type Primitive%20Component%20Object%20Reference) (OtherBodyIndex :type Integer))
  (if (and (Actor|ActorHasTag OtherActor "Player") (Class|CauseOfFire|GetIsActivated))
    (bind _asw_investigation_info (Utilities|Casting|CastToW_InvestigationInfo (UserInterface|GetWidget (Variables|Default|GetWidgetComponent))))
    (Default|PlayAnim _asw_investigation_info false)))

(event EventBeginPlay
  (bind _asw_investigation_info (Utilities|Casting|CastToW_InvestigationInfo (UserInterface|GetWidget (Variables|Default|GetWidgetComponent))))
  (bind _output_get (Variables|Default|SetWidgetRef _asw_investigation_info))
  (Default|SetInfoText _output_get (Variables|Gameplay|GetInfoText)))

(fn ConstructionScript)