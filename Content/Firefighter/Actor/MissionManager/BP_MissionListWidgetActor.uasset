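; World actor that hosts the firefighter mission list widget and relays mission changes to it.
; On BeginPlay it caches the BP_MissionList_ widget from its WidgetComponent, along with the firefighter game mode.
; UpdateMissionList adds or removes missions by ID; adding looks up D_FirefighterMissionData and passes only active rows' text, completion condition and next mission to the widget.
; UpdateMissionData forwards new condition values to the widget.
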(event Custom|UpdateMissionList
  (params (MissionID :type Integer) (bIsRemoveTarget :type Boolean))
  ;[1 1 1] 코멘트
  (if bIsRemoveTarget
    (CallFunction|RemoveMissionfromList MissionID)
    (else
      (CallFunction|AddMissiontoList MissionID))))

(event Custom|AddMissionToList
  (params (NewMissionID :type Integer))
  ;[1 1 1] MissionIdx에 해당하는 미션을 추가한다
  (bind _returnvalue (Utilities|GetDataTableRow "/Game/Firefighter/Data/D_FirefighterMissionData.D_FirefighterMissionData" (Utilities|String|StringToName (Utilities|String|ToString(Integer) NewMissionID)))
    (:then
      (if (.bIsActive (Utilities|Struct|BreakS_FirefighterMission _returnvalue))
        (Default|AddMissiontoList (Variables|Default|GetMissionListRef_) (.Description (Utilities|Struct|BreakS_FirefighterMission _returnvalue)) NewMissionID (.CompleteCondition (Utilities|Struct|BreakS_FirefighterMission _returnvalue)) 0 (.NextMission (Utilities|Struct|BreakS_FirefighterMission _returnvalue)))))))

(event Custom|RemoveMissionFromList
  (params (Target%20Mission%20ID :type Integer))
  ;[1 1 1] MissionIdx에 해당하는 미션을 제거
  (Default|RemoveMissionfromList (Variables|Default|GetMissionListRef_) Target%20Mission%20ID))

(event Custom|UpdateMissionData
  (params (MissionID :type Integer) (NewValue :type Integer))
  (Default|UpdateMission (Variables|Default|GetMissionListRef_) MissionID NewValue))

(event EventBeginPlay
  ;[1 1 1] BeginPlay : MissionList위젯의 ref를 따옴
  (|GetMissionListWidgetRef)
  (|GetGameModeRef))

(fn ConstructionScript)