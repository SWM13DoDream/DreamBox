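; BP_MissionListManager is an actor that relays mission changes to the W_MissionList_ UI held in its widget component, in the Firefighter game.
; On BeginPlay it caches that widget and the game mode, though these graphs never use the latter.
; UpdateMissionList adds missions using D_FirefighterMissionData rows or removes them, always as player 0, while UpdateMissionData forwards new condition values.
; A comment marks it for planned C++ conversion.
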(event Custom|UpdateMissionList
  (params (PlayerID :type Integer) (MissionID :type Integer) (bIsRemoveTarget :type Boolean))
  ;[1 0.6875 0.7889] C++ 전환 예정
  (if bIsRemoveTarget
    (CallFunction|RemoveMissionfromList 0 MissionID)
    (else
      (CallFunction|AddMissiontoList PlayerID MissionID))))

(event Custom|AddMissionToList
  (params (PlayerID :type Integer) (NewMissionID :type Integer))
  ;[1 0.6875 0.7889] C++ 전환 예정
  ;;[1 1 1] MissionIdx에 해당하는 미션을 추가한다
  (bind _returnvalue (Utilities|GetDataTableRow "/Game/Firefighter/Data/D_FirefighterMissionData.D_FirefighterMissionData" (Utilities|String|StringToName (Utilities|String|ToString(Integer) NewMissionID)))
    (:then
      (if true
        (Default|AddMissiontoList (Variables|Default|GetMissionListRef_) PlayerID NewMissionID _returnvalue)))))

(event Custom|RemoveMissionFromList
  (params (PlayerID :type Integer) (Target%20Mission%20ID :type Integer))
  ;[1 0.6875 0.7889] C++ 전환 예정
  ;;[1 1 1] MissionIdx에 해당하는 미션을 제거
  (Default|RemoveMissionfromList (Variables|Default|GetMissionListRef_) 0 Target%20Mission%20ID))

(event Custom|UpdateMissionData
  (params (PlayerID :type Integer) (MissionID :type Integer) (NewValue :type Integer))
  ;[1 0.6875 0.7889] C++ 전환 예정
  (Default|UpdateMission (Variables|Default|GetMissionListRef_) PlayerID MissionID NewValue))

(event EventBeginPlay
  ;[1 0.6875 0.7889] C++ 전환 예정
  ;;[1 1 1] BeginPlay : MissionList위젯의 ref를 따옴
  (|GetMissionListWidgetRef)
  (|GetGameModeRef))

(fn ConstructionScript)