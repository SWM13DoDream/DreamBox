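; BP_MissionTrigger is a placeable trigger that updates the player's mission list in the firefighter game.
; On BeginPlay it caches the game mode and player, and, if IsAutoActivate is set, sends the update after a short delay.
; A Player-tagged actor overlapping TriggerBox also sends it, then destroys the trigger.
; Updates go through the game mode's CallUpdateMissionList with MissionID and IsRemoveTarget, always for player 0.
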(event OnComponentBeginOverlap(TriggerBox)
  (params (OverlappedComponent :type Primitive%20Component%20Object%20Reference) (OtherActor :type Actor%20Object%20Reference) (OtherComp :type Primitive%20Component%20Object%20Reference) (OtherBodyIndex :type Integer) (bFromSweep :type Boolean) (SweepResult :type Hit%20Result%20Structure%20%28by%20ref%29))
  (|CheckActorIsPlayer&Valid OtherActor
    (:True
      (CallFunction|UpdateMissionDelegate)
      (Development|PrintString "Trigger")
      (Actor|DestroyActor))))

(event Custom|UpdateMissionDelegate
  (Default|CallUpdateMissionList (Variables|Reference|GetGameModeRef) 0 (Variables|Default|GetMissionID) (Variables|Default|GetIs%20Remove%20Target)))

(event EventBeginPlay
  (|GetGameModeRef)
  (|GetPlayerRef)
  (if (Variables|Default|GetbIsAutoActivate)
    (Utilities|FlowControl|Delay 0.2)
    (CallFunction|UpdateMissionDelegate)))

(fn ConstructionScript)