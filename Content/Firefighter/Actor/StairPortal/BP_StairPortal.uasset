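; Stair portal that teleports the VR player to a linked previous or next point on entering its trigger volume.
; The length of its Direction vector plus normalized player velocity determines backward or forward travel.
; It requests a game mode fade, waits briefly, moves the capsule, then adds yaw input.
; GetNextTransform derives the destination from the target's Direction, flipping yaw and raising height for forward travel.
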(event OnComponentBeginOverlap(TriggerVolume)
  (params (OverlappedComponent :type Primitive%20Component%20Object%20Reference) (OtherActor :type Actor%20Object%20Reference) (OtherComp :type Primitive%20Component%20Object%20Reference) (OtherBodyIndex :type Integer) (bFromSweep :type Boolean) (SweepResult :type Hit%20Result%20Structure%20%28by%20ref%29))
  (bind _nextpoint (Variables|Default|GetNextPoint))
  (bind _prevpoint (Variables|Default|GetPrevPoint))
  (if (Actor|ActorHasTag OtherActor "Player")
    (bind _asvrcharacter (Utilities|Casting|CastToVRCharacter OtherActor))
    (Development|PrintString (Utilities|String|ToString(Float) (Math|Vector|VectorLength (+ (Math|Vector|GetForwardVector (Variables|Default|GetDirection)) (Math|Vector|Normalize (Variables|/Script/Engine.MovementComponent|GetVelocity (Pawn|GetMovementComponent _asvrcharacter)))))))
    (switch int (Math|Conversions|ToInteger(Byte) (Class|KismetMathLibrary|FTrunc64 (Math|Vector|VectorLength (+ (Math|Vector|GetForwardVector (Variables|Default|GetDirection)) (Math|Vector|Normalize (Variables|/Script/Engine.MovementComponent|GetVelocity (Pawn|GetMovementComponent _asvrcharacter))))))) ; 0이면 반대, 1이면 같은 방향
      (:0
        (Utilities|IsValid _prevpoint
          (:Is%20Valid
            (Default|CallPlayFadeinOutAnimation (Variables|Default|GetGamemodeRef))
            (Utilities|FlowControl|Delay 0.75)
            (Transformation|SetWorldTransform (Variables|/Script/Engine.Character|GetCapsuleComponent _asvrcharacter) (CallFunction|GetNextTransform true _prevpoint) false true))))
      (:1
        (Utilities|IsValid _nextpoint :!label _label
          (:Is%20Valid
            (Default|CallPlayFadeinOutAnimation (Variables|Default|GetGamemodeRef))
            (Utilities|FlowControl|Delay 0.75)
            (Transformation|SetWorldTransform (Variables|/Script/Engine.Character|GetCapsuleComponent _asvrcharacter) (CallFunction|GetNextTransform false _nextpoint) false true))))
      (:2
        (goto _label)))
    (Pawn|Input|AddControllerYawInput _asvrcharacter 72.5)))

(event EventBeginPlay
  (bind _asbp_firefighter_game_mode (Utilities|Casting|CastToBP_FirefighterGameMode (Game|GetGameMode)))
  (Variables|Default|SetGamemodeRef _asbp_firefighter_game_mode))

(fn ConstructionScript)

(fn GetNextTransform
  (params (bIsBack :type Boolean) (Target :type BP%20Stair%20Portal%20Object%20Reference))
  (bind _returnvalue (Math|Integer|SelectInt 0 180 bIsBack))
  (bind _direction (Variables|BP_StairPortal_C|GetDirection Target))
  (bind _returnvalue_2 (Transformation|GetWorldRotation _direction))
  (bind _returnvalue_3 (Math|Conversions|ToFloat(Integer) _returnvalue))
  (bind (_roll _pitch _yaw) (Math|Rotator|BreakRotator _returnvalue_2))
  (bind _returnvalue_4 (+ _yaw _returnvalue_3))
  (bind _returnvalue_5 (Math|Float|%(Float) _returnvalue_4 3.6e+02))
  (bind _returnvalue_6 (Math|Rotator|MakeRotator _roll _pitch _returnvalue_5))
  (Development|PrintString (Utilities|String|ToString(Rotator) _returnvalue_6))
  (return (Math|Transform|MakeTransform (+ (+ (Transformation|GetWorldLocation _direction) (* (Math|Vector|GetForwardVector _returnvalue_6) (Math|Conversions|ToFloat(Integer) (Math|Integer|SelectInt -100 -100 bIsBack)))) (Math|Vector|SelectVector "0, 0, 0" "0.000000,0.000000,140.000000" bIsBack)) _returnvalue_6)))