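; BP_ScriptManager is an actor that displays script lines for a given player in the firefighter game and plays voice dubbing for them.
; On BeginPlay it caches the W_Script widget from its Widget component.
; Showing a script by ID updates that widget, then restarts the VoiceDubbing audio with its Index parameter set to the ID.
; Showing a script by string only updates the widget, without audio.
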(event Custom|ShowScriptWithID
  (params (PlayerID :type Integer) (ScriptID :type Integer))
  (bind _voicedubbing (Variables|Default|GetVoiceDubbing))
  (Default|ShowScriptwithID (Variables|Default|GetScriptWidgetRef) PlayerID ScriptID)
  (Audio|Components|Audio|Stop _voicedubbing)
  (Effects|Components|ParticleSystem|SetIntParameter _voicedubbing "Index" ScriptID)
  (Audio|Components|Audio|Play _voicedubbing 0.0))

(event Custom|ShowScriptWithString
  (params (PlayerID :type Integer) (Script :type String))
  (Default|ShowScriptwithString (Variables|Default|GetScriptWidgetRef) PlayerID Script))

(event EventBeginPlay
  (|GetScriptWidgetRef))

(fn ConstructionScript)