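; Firefighter player character that relays game mode events to its mission list and script displays.
; On BeginPlay it caches the game mode and the two child-actor widget managers, then binds its handlers to game mode delegates.
; Mission and script-by-ID handlers forward with player ID fixed to 0, while script-by-string passes it through.
; CrossFade calls a player index check, then plays the game mode's fade sequence while briefly deactivating movement.
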(event Custom|UpdateMissionList
  (params (PlayerID :type Integer) (MissionID :type Integer) (bIsRemoveTarget :type Boolean))
  ;[1 0.8939 0.4913] Widget Event : 소유한 위젯 액터의 업데이트 함수를 호출
  ;;[1 0.8065 0.5083] 미션 리스트를 업데이트 (추가 및 제거)
  (Default|UpdateMissionList (Variables|Default|GetMissionWidgetRef) 0 MissionID bIsRemoveTarget))

(event Custom|UpdateMissionData
  (params (PlayerID :type Integer) (MissionID :type Integer) (NewCondition :type Integer))
  ;[1 0.8939 0.4913] Widget Event : 소유한 위젯 액터의 업데이트 함수를 호출
  ;;[1 0.6548 0.4927] 특정 미션을 업데이트
  (Default|UpdateMissionData (Variables|Default|GetMissionWidgetRef) 0 MissionID NewCondition))

(event Custom|ShowScriptWithID
  (params (PlayerID :type Integer) (ScriptID :type Integer))
  ;[1 0.8939 0.4913] Widget Event : 소유한 위젯 액터의 업데이트 함수를 호출
  ;;[1 0.6399 0.3618] 특정 스크립트를 출력 (데이터 테이블 기반
  (Default|ShowScriptwithID (Variables|Default|GetScriptWidgetRef) 0 ScriptID))

(event Custom|ShowScriptWithString
  (params (PlayerID :type Integer) (Script :type String))
  ;[1 0.8939 0.4913] Widget Event : 소유한 위젯 액터의 업데이트 함수를 호출
  ;;[0.4072 0.2623 0.147] 특정 스크립트를 출력 (임의의 스트링
  (Default|ShowScriptwithString (Variables|Default|GetScriptWidgetRef) PlayerID Script))

(event Custom|CrossFade
  (params (PlayerID :type Integer))
  ;[1 0.8939 0.4913] Widget Event : 소유한 위젯 액터의 업데이트 함수를 호출
  ;;[1 1 1] 페이드 인 아웃 이벤트
  (|CheckPlayerIdx PlayerID)
  (Components|Activation|Deactivate (Variables|Character|GetCharacterMovement))
  (Sequencer|Player|Play (Variables|/Game/Firefighter/BP_FireFIghterGameMode.BP_FirefighterGameMode_C|GetCrossFadeSQRef (Variables|Default|GetGameModeRef_0)) :!class /Script/MovieScene.MovieSceneSequencePlayer)
  (Utilities|FlowControl|Delay 1.25)
  (Components|Activation|Activate (Variables|Character|GetCharacterMovement) false))

(event EventBeginPlay
  ;[0.9606 0.1568 1] BeginPlay 이벤트
  (|GetGameModeRef)
  (|GetMissionWidgetRef)
  (|BindToDelegate (delegate Custom|UpdateMissionList) (delegate Custom|UpdateMissionData) (delegate Custom|ShowScriptWithID) (delegate Custom|CrossFade) (delegate Custom|ShowScriptWithString)))

(fn ConstructionScript)