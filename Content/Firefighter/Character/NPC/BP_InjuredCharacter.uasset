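; BP_InjuredCharacter is an injured NPC in a firefighter game that displays a rescue control prompt when the player comes near.
; Entering its InteractionTrigger while no rescue is under way makes the InfoWidget component visible and plays the W_ControlGuide_Rescue animation.
; Leaving the trigger calls the same animation function with false, without changing the component's visibility.
; The rescue state comes from GetIsBeingRescued, and construction only runs the parent script.
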(event OnComponentBeginOverlap(InteractionTrigger)
  (params (OverlappedComponent :type Primitive%20Component%20Object%20Reference) (OtherActor :type Actor%20Object%20Reference) (OtherComp :type Primitive%20Component%20Object%20Reference) (OtherBodyIndex :type Integer) (bFromSweep :type Boolean) (SweepResult :type Hit%20Result%20Structure%20%28by%20ref%29))
  (bind _infowidget (Variables|Default|GetInfoWidget))
  (if (and (Actor|ActorHasTag OtherActor "Player") (not (Class|InjuredCharacter|GetIsBeingRescued)))
    (bind _asw_control_guide_rescue (Utilities|Casting|CastToW_ControlGuide_Rescue (UserInterface|GetWidget _infowidget)))
    (Rendering|SetVisibility _infowidget true false)
    (Default|PlayAnim _asw_control_guide_rescue true)))

(event OnComponentEndOverlap(InteractionTrigger)
  (params (OverlappedComponent :type Primitive%20Component%20Object%20Reference) (OtherActor :type Actor%20Object%20Reference) (OtherComp :type Primitive%20Component%20Object%20Reference) (OtherBodyIndex :type Integer))
  (if (Actor|ActorHasTag OtherActor "Player")
    (bind _asw_control_guide_rescue (Utilities|Casting|CastToW_ControlGuide_Rescue (UserInterface|GetWidget (Variables|Default|GetInfoWidget))))
    (Default|PlayAnim _asw_control_guide_rescue false)))

(fn ConstructionScript
  (|CallParentFunction))