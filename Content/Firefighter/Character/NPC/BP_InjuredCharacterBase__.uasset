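; Base Blueprint for injured NPC characters in the firefighter game, assembled from modular skeletal parts and hand-held static meshes.
; The Construction Script makes parts follow the main mesh's pose, attaches hand meshes to sockets, and sets hat and glove morph targets.
; The animation-mode check has unconnected logic, so morphs always go through each part's AnimInstance and the BeginPlay reapply for single-animation mode never fires.
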(event EventBeginPlay
  ;[1 1 1] Update Morph Targets again, since we can not set them in Construction Script with Animation Mode "Use Animation Asset"
  (if (CallFunction|IsDefaultMeshInheritungItsAnimationAsset)
    (CallFunction|UpdateMorphTargets)))

(fn ConstructionScript
  (Variables|Customization|SetRefresh false)
  (CallFunction|UpdateMorphTargets)
  (CallFunction|SetMasterPoseComponentforParts))

(fn SetMasterPoseComponentforParts
  ;[0 0 0] Updates all Part components (skeletal and static meshes) to follow the Master Pose of Mesh (Inherited).
  ;
  ; This means, you can set the character's animation in its editor Details Panel or in Mesh (Inherited) component itself, which then gets used for all other Part components as well automatically.
  (Class|SkinnedMeshComponent|SetMasterPoseComponent (Variables|Default|GetSK_Eyeglasses) (Variables|Character|GetMesh) false)
  (Transformation|AttachComponentToComponent (Variables|Default|GetSM_LeftHand) (Variables|Character|GetMesh) "LeftHandSocket" "KeepRelative" "KeepRelative" "KeepRelative" true)
  (Transformation|AttachComponentToComponent (Variables|Default|GetSM_RightHand) (Variables|Character|GetMesh) "RightHandSocket" "KeepRelative" "KeepRelative" "KeepRelative" true))

(fn IsDefaultMeshInheritungItsAnimationAsset)

(fn GetMorphTargetValue
  (params (CanMorph :type Boolean))
  (return (Math|Float|SelectFloat 1.0 0.0 CanMorph)))

(fn UpdateMorphTargets
  (bind _sk_hair (Variables|Default|GetSK_Hair))
  (bind _sk_hat (Variables|Default|GetSK_Hat))
  (bind _sk_head (Variables|Default|GetSK_Head))
  (bind _sk_hand_glove (Variables|Default|GetSK_Hand/Glove))
  (bind _sk_eyeglasses (Variables|Default|GetSK_Eyeglasses))
  (bind _sk_chest (Variables|Default|GetSK_Chest))
  (bind _array (Utilities|Array|MakeArray _sk_hat _sk_hair _sk_head _sk_chest _sk_hand_glove _sk_eyeglasses))
  (if (CallFunction|IsDefaultMeshInheritungItsAnimationAsset)
    (Components|SkeletalMesh|SetMorphTarget _array "hat_equipped" (CallFunction|GetMorphTargetValue (Variables|Customization|MorphTargets|GetHatEquipped)) true)
    (Components|SkeletalMesh|SetMorphTarget _array "gloves_equipped" (CallFunction|GetMorphTargetValue (Variables|Customization|MorphTargets|GetGlovesEquipped)) true)
    (else
      (for _array_element _array
        (Utilities|IsValid _array_element
          (:Is%20Valid
            (Utilities|IsValid (Components|SkeletalMesh|GetAnimInstance _array_element)
              (:Is%20Valid
                (Components|SkeletalMesh|SetMorphTarget (Components|SkeletalMesh|GetAnimInstance _array_element) "hat_equipped" (CallFunction|GetMorphTargetValue (Variables|Customization|MorphTargets|GetHatEquipped)))
                (Components|SkeletalMesh|SetMorphTarget (Components|SkeletalMesh|GetAnimInstance _array_element) "gloves_equipped" (CallFunction|GetMorphTargetValue (Variables|Customization|MorphTargets|GetGlovesEquipped)))))))))))